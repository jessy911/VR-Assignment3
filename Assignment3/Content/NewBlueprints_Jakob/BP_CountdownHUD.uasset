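; BP_CountdownHUD is a world-space HUD actor, named for a countdown, that floats in front of the VR player's view.
; Every tick it computes a transform from the VRPawn's camera and snaps itself there, a fixed distance along the camera's forward vector.
; A look-at rotation from its root toward the camera keeps it facing the player.
; The graphs contain only this follow behavior, with no countdown logic.
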(event EventTick
  (params (DeltaSeconds :type Float%20%28single-precision%29))
  (Utilities|IsValid (Variables|Default|GetDefaultSceneRoot)
    (:Is%20Valid
      (bind _hudtransform (CallFunction|GetHUDTransform))
      (Transformation|SetActorTransform _hudtransform))))

(fn ConstructionScript)

(fn GetHUDTransform
  (bind _asvrpawn (Utilities|Casting|CastToVRPawn (Game|Player|GetPlayerPawn 0)))
  (return (Math|Transform|MakeTransform (+ (* (Math|Vector|GetForwardVector (Variables|/Game/VRTemplate/Blueprints/VRPawn.VRPawn_C|GetCamera _asvrpawn)) 400) (Transformation|GetWorldLocation (Variables|/Game/VRTemplate/Blueprints/VRPawn.VRPawn_C|GetCamera _asvrpawn))) (Math|Rotator|FindLookatRotation (Transformation|GetWorldLocation (Variables|Default|GetDefaultSceneRoot)) (Transformation|GetWorldLocation (Variables|/Game/VRTemplate/Blueprints/VRPawn.VRPawn_C|GetCamera _asvrpawn))))))