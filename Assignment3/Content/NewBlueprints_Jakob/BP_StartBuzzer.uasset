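; BP_StartBuzzer is a VR race start button that starts the timer once every buzzer in the level is active.
; A VRPawn overlap presses the button, plays a click and checks all BP_StartBuzzer actors.
; If all are active, their column materials get the race color and StartTimer is sent; otherwise this one stays active for DelayTime.
; The color reset targets \"ColumnColorNone\", and the node applying the dynamic material never runs.
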(event OnComponentBeginOverlap(Box)
  (params (OverlappedComponent :type Primitive%20Component%20Object%20Reference) (OtherActor :type Actor%20Object%20Reference) (OtherComp :type Primitive%20Component%20Object%20Reference) (OtherBodyIndex :type Integer) (bFromSweep :type Boolean) (SweepResult :type Hit%20Result%20Structure%20%28by%20ref%29))
  (bind _button (Variables|Default|GetButton))
  (Utilities|Casting|CastToVRPawn OtherActor)
  (Components|MoveComponentTo _button (- (Variables|Default|GetStartLocation) "0.000000,0.000000,0.350000") "0, 0, 0" false false 0.1 false)
  (Development|PrintString "workin?" true true "(R=1.000000,G=0.456561,B=0.231010,A=1.000000)" 1e+02)
  (Class|BPIInteraction|Interact(Message) _button)
  (Audio|PlaySound2D "/Engine/VREditor/Sounds/UI/Click_on_Button.Click_on_Button" 1.0 1.0 0.0 0 0)
  ;[0.15 0.15 0.15 0.5] Check if both Buttons are active
  (Variables|Default|SetButtonActive true)
  (bind _outactors (Actor|GetAllActorsOfClass "BP_StartBuzzer_C"))
  (Variables|Default|SetStartCountDown true)
  (for _array_element _outactors
    (if (== (Variables|BP_StartBuzzer_C|GetButtonActive _array_element) false)
      (Variables|Default|SetStartCountDown false)))
  (if (Variables|Default|GetStartCountDown)
    ;[0.15 0.15 0.15 0.5] Both Buttons are Active -> Race is starting
    (bind _outactors_2 (Actor|GetAllActorsOfClass "BP_StartBuzzer_C"))
    (for _array_element_2 _outactors_2
      (Rendering|Material|SetVectorParameterValue (Variables|BP_StartBuzzer_C|GetColumnMaterial _array_element_2) "ColumnColor" (Math|Conversions|ToLinearColor(Color) (Variables|Default|GetColumnRaceColor)) :!class /Script/Engine.MaterialInstanceDynamic))
    (Class|BPIStartTimer|StartTimer(Message) (Utilities|ToObject(Interface) (Variables|Default|GetBPI_StartTimerRef)))
    (else
      ;[0.15 0.15 0.15 0.5] Only One Button is active
      (Rendering|Material|SetVectorParameterValue (Variables|Default|GetColumnMaterial) "ColumnColor" (Math|Conversions|ToLinearColor(Color) (Variables|Default|GetColumnActiveColor)) :!class /Script/Engine.MaterialInstanceDynamic)
      (Utilities|FlowControl|Delay (Variables|Default|GetDelayTime))
      (Variables|Default|SetButtonActive false)
      (Rendering|Material|SetVectorParameterValue (Variables|Default|GetColumnMaterial) "ColumnColorNone" (Math|Conversions|ToLinearColor(Color) (Variables|Default|GetColumnBaseColor)) :!class /Script/Engine.MaterialInstanceDynamic)
      (Development|PrintString "ColorChanged" true true "(R=0.000000,G=1.000000,B=0.304781,A=1.000000)" 1e+02))))

(event OnComponentEndOverlap(Button)
  (params (OverlappedComponent :type Primitive%20Component%20Object%20Reference) (OtherActor :type Actor%20Object%20Reference) (OtherComp :type Primitive%20Component%20Object%20Reference) (OtherBodyIndex :type Integer))
  (Utilities|Casting|CastToVRPawn OtherActor)
  (Utilities|FlowControl|Delay 0.1)
  (Components|MoveComponentTo (Variables|Default|GetButton) (Variables|Default|GetStartLocation) "0, 0, 0" false false 0.1 false))

(event EventBeginPlay
  (Variables|Default|SetStartLocation (Variables|/Script/Engine.SceneComponent|GetRelativeLocation (Variables|Default|GetButton)))
  (bind _returnvalue (Rendering|Material|CreateDynamicMaterialInstance "/Game/NewMaterials_Jakob/M_BuzzerColumn.M_BuzzerColumn" "None" "None" :!class /Script/Engine.KismetMaterialLibrary))
  (bind _output_get (Variables|Default|SetColumnMaterial _returnvalue))
  (Rendering|Material|SetVectorParameterValue _output_get "ColumnColor" (Math|Conversions|ToLinearColor(Color) (Variables|Default|GetColumnBaseColor)) :!class /Script/Engine.MaterialInstanceDynamic))

(event EventInteract)

(fn ConstructionScript)